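; BP_Tile is a tile actor that asks the Blueprint manager to construct a random tile when the player's test pawn enters its trigger box.
; On BeginPlay it fetches the manager reference from the game mode, polling with a short delay until it is valid.
; The first pawn overlap shuffles TileTable, prints the first entry and passes it with the actor's location to CallConstructionTile, guarded by DoOnce.
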(event `self.ReceiveBeginPlay`
  (bind _asmy_game_mode (cast `/Game/blueprint/management/my_game_mode` (`GameplayStatics.GetGameMode`)))
  (bind _output_get (set `self.Ref BP Manager` (`/Game/blueprint/management/my_game_mode.Ref_BP_Manager` _asmy_game_mode) :!label _label))
  (`/Engine/EditorBlueprintResources/StandardMacros.IsValid` _output_get
    (:`Is Not Valid`
      (`KismetSystemLibrary.Delay` 0.02)
      (goto _label))))

(event `self.Box.OnComponentBeginOverlap`
  (params (OverlappedComponent :type "PrimitiveComponent Object Reference") (OtherActor :type "Actor Object Reference") (OtherComp :type "PrimitiveComponent Object Reference") (OtherBodyIndex :type Integer) (bFromSweep :type Boolean) (SweepResult :type "HitResult Structure (by ref)"))
  (bind _tile_table (`self.Tile_Table`))
  (bind _output (`|GetArrayItem` _tile_table))
  (cast `/Game/blueprint/pawn/pawn_test` OtherActor)
  (`/Engine/EditorBlueprintResources/StandardMacros.DoOnce` false
    (:`Completed`
      (`KismetArrayLibrary.Array_Shuffle` _tile_table)
      (`KismetSystemLibrary.PrintString` (`KismetStringLibrary.Conv_IntToString` _output))
      (`/Game/Etudiant/Tiles/BP_Manager.Call_Construction_Tile` (`self.Ref BP Manager`) (`self.K2_GetActorLocation`) _output))))

(fn `UserConstructionScript`)