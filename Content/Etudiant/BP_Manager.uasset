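; BP_Manager spawns level tiles on request and caps how many exist at once.
; Call_Construction_Tile takes a one-based index into TileChoice and spawns that class at Position, offset along X by TileSpace times TileSize.
; Each tile is appended to TileList; beyond 150 entries, the oldest is destroyed and removed, with a debug print.
; Tick and BeginPlay are unused, and this graph never updates the placement variables.
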(event `Call_Construction_Tile`
  (params (Position :type "Vector Structure") (Tile_Index :type Integer))
  (bind _tile_list (`self.Tile_List`))
  (bind _tile_list_2 (`self.Tile_List`))
  (bind _returnvalue (`|SpawnActorFromClass` (`|GetArrayItem` (`self.Tile_Choice`) (- Tile_Index 1)) (`KismetMathLibrary.MakeTransform` (`KismetMathLibrary.MakeVector` (+ Position_X (* (`self.Tile_Space`) (`self.Tile_Size`))) Position_Y Position_Z)) "Undefined" "MultiplyWithRoot" null null))
  (`KismetArrayLibrary.Array_Add` _tile_list_2 _returnvalue)
  (if (> (`KismetArrayLibrary.Array_Length` _tile_list_2) 150)
    (`KismetSystemLibrary.PrintString` "test")
    (`self.K2_DestroyActor` (`|GetArrayItem` _tile_list))
    (`KismetArrayLibrary.Array_Remove` _tile_list)))

(fn `UserConstructionScript`)